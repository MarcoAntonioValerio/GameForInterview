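; Player Blueprint for 2D flipbook movement with run and idle animations.
; Vertical and horizontal axis inputs apply impulses on Z and X to the Player flipbook component, scaled by PlayerSpeed and delta time.
; Only the vertical input updates AmIMoving, so horizontal movement alone does not trigger the run animation.
; Tick calls AnimationContoller, which picks the run or idle flipbook from that flag.
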(event `self.ReceiveTick`
  (params (DeltaSeconds :type "Float (single-precision)"))
  (`self.AnimationContoller`))

(event `InputAxis|VerticalMovementInput`
  (params (AxisValue :type "Float (single-precision)"))
  ;[1 1 1] Movement Inputs
  ;;[1 1 1] Adds Impulse on the Z azis.
  (`PrimitiveComponent.AddImpulse` (`self.Player`) (`KismetMathLibrary.MakeVector` 0.0 0.0 (* (* (`self.PlayerSpeed`) AxisValue (`GameplayStatics.GetWorldDeltaSeconds`)) 100.0)) "None" false)
  (if (or (!= AxisValue 0.0) (!= (stale `InputAxis|HorizontalMovementImput` AxisValue) 0.0))
    (set `self.AmIMoving` true)
    (else
      (set `self.AmIMoving` false))))

(event `InputAxis|HorizontalMovementImput`
  (params (AxisValue :type "Float (single-precision)"))
  ;[1 1 1] Movement Inputs
  ;;[1 1 1] Adds Impulse on the Z azis.
  (`PrimitiveComponent.AddImpulse` (`self.Player`) (`KismetMathLibrary.MakeVector` (* (* (`self.PlayerSpeed`) AxisValue (`GameplayStatics.GetWorldDeltaSeconds`)) 100.0)) "None" false))

(event `AnimationContoller`
  ;[1 1 1] Checks If I am moving
  (if (`self.AmIMoving`)
    (`PaperFlipbookComponent.SetFlipbook` (`self.Player`) "/Game/Sprites/PlayerSprites/anim_Run.anim_Run")
    (else
      (`PaperFlipbookComponent.SetFlipbook` (`self.Player`) "/Game/Sprites/PlayerSprites/anim_Idle.anim_Idle"))))

(fn `UserConstructionScript`)